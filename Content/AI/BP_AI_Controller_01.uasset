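; AI controller that wanders its pawn and steers it away from obstacles with a simple sense-decide-move loop on Tick.
; A debug-drawn visibility line trace probes a short distance along the pawn's forward vector.
; While the trace hits, the stored Direction vector rotates by a small fixed step each frame.
; The pawn receives reduced-scale movement input along Direction every frame, whether blocked or not.
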(event `self.ReceiveTick`
  (params (DeltaSeconds :type "Float (single-precision)"))
  (bind _returnvalue (`self.K2_GetPawn`))
  (bind _returnvalue_2 (`self.K2_GetActorLocation` _returnvalue))
  ;[1 1 1] Зрение
  (bind (_outhit _returnvalue_3) (`KismetSystemLibrary.LineTraceSingle` :`Start` _returnvalue_2 :`End` (+ _returnvalue_2 (* (`self.GetActorForwardVector` _returnvalue) 800)) :`TraceChannel` "TraceTypeQuery1" :`DrawDebugType` "ForOneFrame"))
  ;[1 1 1] Мозг
  (if _returnvalue_3
    (set `self.Direction` (`KismetMathLibrary.GreaterGreater_VectorRotator` (`self.Direction`) (struct :`Yaw` 1.0))))
  ;[1 1 1] Ноги
  (`Pawn.AddMovementInput` (`self.K2_GetPawn`) (`self.Direction`) 0.7 false))

(fn `UserConstructionScript`)