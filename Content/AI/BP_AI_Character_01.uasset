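; BP_AI_Character_01 is a simple AI character that wanders and steers away from obstacles, without an AI controller or navigation calls in its graph.
; Each Tick runs a sense-decide-act loop, starting with a debug-drawn Visibility line trace ahead along the actor's forward vector.
; A hit rotates the stored Direction vector by a small fixed step per frame, so turn rate depends on framerate.
; Movement input is applied continuously along Direction at reduced scale.
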(event `self.ReceiveTick`
  (params (DeltaSeconds :type "Float (single-precision)"))
  (bind _returnvalue (`self.K2_GetActorLocation`))
  ;[1 1 1] Зрение
  (bind (_outhit _returnvalue_2) (`KismetSystemLibrary.LineTraceSingle` :`Start` _returnvalue :`End` (+ _returnvalue (* (`self.GetActorForwardVector`) 800)) :`TraceChannel` "TraceTypeQuery1" :`DrawDebugType` "ForOneFrame"))
  ;[1 1 1] Мозг
  (if _returnvalue_2
    (set `self.Direction` (`KismetMathLibrary.GreaterGreater_VectorRotator` (`self.Direction`) (struct :`Yaw` 1.0))))
  ;[1 1 1] Ноги
  (`self.AddMovementInput` (`self.Direction`) 0.3))

(fn `UserConstructionScript`)