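; AI controller for an enemy that patrols randomly around its spawn point, investigates noises and chases targets it sees or is damaged by.
; Player controller events toggle movement and perception while it is alive; zero health stops it permanently.
; Patrol and chase loop by re-calling themselves on each successful move.
; Hearing sends it near the noise, gated until arrival, and losing sight resumes patrol after a pause.
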(event `Patrolling`
  ;[1 1 1] Patrolling
  (if (`self.bCanMove`)
    (`|AIMoveTo` null (`NavigationSystemV1.K2_GetRandomReachablePointInRadius` (`self.SpawnPoint`) 2000.0 null null) null
      (:`OnSuccess`
        (`self.Patrolling`)))))

(event `self.ReceiveBeginPlay`
  ;[1 1 1] Save patrol location
  (set `self.SpawnPoint` (`self.K2_GetActorLocation` (`self.K2_GetPawn`)))
  ;[1 1 1] Start/Stop AI
  (bind _outactors (`GameplayStatics.GetAllActorsOfClass` "/Game/ThirdPerson/Blueprints/BP_PlayerController.BP_PlayerController_C"))
  (for _array_element _outactors
    (add `/Game/ThirdPerson/Blueprints/BP_PlayerController.CanMoveAI` _array_element (delegate `CanMoveAI_Event`))))

(event `CanMoveAI_Event`
  (bind _aiperception (`self.AIPerception`))
  ;[1 1 1] Start/Stop AI
  (if (`self.bIsAlive`)
    (bind _output_get (set `self.bCanMove` (not (`self.bCanMove`))))
    (if _output_get
      (`ActorComponent.Activate` _aiperception true)
      (`self.Patrolling`)
      (else
        (`ActorComponent.Deactivate` _aiperception)
        (`self.StopMovement`)))))

(event `self.AIPerception.OnTargetPerceptionUpdated`
  (params (Actor :type "Actor Object Reference") (Stimulus :type "AIStimulus Structure"))
  (bind (_age _expirationage _strength _stimuluslocation _receiverlocation _tag _bsuccessfullysensed) (break `AIStimulus` Stimulus))
  (if (`self.bCanMove`)
    (bind _returnvalue (`AIPerceptionSystem.GetSenseClassForStimulus` Stimulus))
    (switch `string` (`KismetSystemLibrary.GetClassDisplayName` _returnvalue)
      (:`AISense_Hearing`
        ;[1 1 1] Check noise
        (if (`self.bCanCheckNoise`)
          (set `self.bCanCheckNoise` false)
          (`self.StopMovement`)
          (`|AIMoveTo` self null (`NavigationSystemV1.K2_GetRandomReachablePointInRadius` _stimuluslocation 1000.0 null null) null 50.0
            (:`OnSuccess`
              (set `self.bCanCheckNoise` true)
              (`KismetSystemLibrary.Delay` 3.0)
              (`self.Patrolling`)))))
      (:`AISense_Sight`
        (if _bsuccessfullysensed
          (`self.ChaseThePlayer` Actor)
          (else
            (`self.StopMovement`)
            (`KismetSystemLibrary.Delay` 2.0)
            (`self.Patrolling`)))))))

(event `ChaseThePlayer`
  (params (TargetPlayer :type "Actor Object Reference"))
  ;[1 1 1] ChaseThePlayer
  (`|AIMoveTo` null (0.0 0.0 0.0) TargetPlayer
    (:`OnSuccess`
      (`KismetSystemLibrary.Delay` 0.2)
      (`self.ChaseThePlayer` TargetPlayer))))

(event `self.ReceiveAnyDamage`
  (params (Damage :type "Float (single-precision)") (DamageType :type "DamageType Object Reference") (InstigatedBy :type "Controller Object Reference") (DamageCauser :type "Actor Object Reference"))
  (bind _output_get (set `self.Health` (- (`self.Health`) Damage)))
  (if (<= _output_get 0.0)
    (set `self.bIsAlive` false)
    (set `self.bCanMove` false)
    (`self.StopMovement`)
    (else
      (`self.ChaseThePlayer` DamageCauser))))

(fn `UserConstructionScript`)